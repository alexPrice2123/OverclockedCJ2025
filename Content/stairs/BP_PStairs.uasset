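; BP_PStairs is a procedural staircase actor that builds its mesh with Geometry Script on rebuild.
; It derives step count from Corner.Z and step height, and step depth and width from Corner's X and Y.
; It appends a base box, then loops overlapping boxes at stepped heights, updating collision after each.
; Counts at or above StairMax get only the base box, and step depth prints for debugging.
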(event `self.OnRebuildGeneratedMesh`
  (params (TargetMesh :type "DynamicMesh Object Reference"))
  (bind (_corner_x _corner_y _corner_z) (`KismetMathLibrary.BreakVector` (`self.Corner`)))
  (bind _corner_x_2 (`KismetMathLibrary.BreakVector` (`self.Corner`)))
  (bind _corner_x_3 (`KismetMathLibrary.BreakVector` (`self.Corner`)))
  (bind _returnvalue (* _corner_x 2.0))
  (bind _returnvalue_2 (- (`self.Step Amount`) 1))
  (set `self.Target Mesh` TargetMesh)
  (bind _output_get (set `self.Step Amount` (`KismetMathLibrary.Round` (/ _corner_z (`self.StepHeight`)))))
  (set `self.Base X` _returnvalue)
  (set `self.Base Y` (* _corner_y 2.0))
  (bind _output_get_2 (set `self.Step X` (/ _returnvalue _output_get)))
  (`KismetSystemLibrary.PrintString` (`KismetStringLibrary.Conv_DoubleToString` _output_get_2))
  (if (> (`self.Step Amount`) 0)
    (bind _returnvalue_3 (`GeometryScriptLibrary_MeshPrimitiveFunctions.AppendBox` (`self.Target Mesh`) (make `GeometryScriptPrimitiveOptions` "SingleGroup") (`KismetMathLibrary.MakeTransform` (`KismetMathLibrary.MakeVector` (* _corner_x_3 -1.0)) (struct) (1.0 1.0 1.0)) (+ (`self.Step X`) (/ (`self.Step X`) 2.0)) (`self.Base Y`) (`self.StepHeight`) 0 0 0 "Base" null)) ; Staur Base
    (`GeometryScriptLibrary_CollisionFunctions.SetDynamicMeshCollisionFromMesh` _returnvalue_3 (`self.DynamicMeshComponent`) (struct) null)
    (if (>= (`self.Step Amount`) (`self.StairMax`))
      _
      (elif (> (`self.Step Amount`) 1)
        ;[0.4531 1 1 0.588] Loop each step - 1
        (for _index (range 1 (+ _returnvalue_2 1))
          (bind _returnvalue_4 (`GeometryScriptLibrary_MeshPrimitiveFunctions.AppendBox` (`self.Target Mesh`) (make `GeometryScriptPrimitiveOptions` "SingleGroup") (`KismetMathLibrary.MakeTransform` (`KismetMathLibrary.MakeVector` (- _corner_x_2 (* _index (`self.Step X`))) 0.0 (+ (* (- _returnvalue_2 _index) (`self.StepHeight`)) (`self.StepHeight`)))) (+ (`self.Step X`) (/ (`self.Step X`) 2.0)) (`self.Base Y`) (`self.StepHeight`) 0 0 0 "Base" null))
          (`GeometryScriptLibrary_CollisionFunctions.SetDynamicMeshCollisionFromMesh` _returnvalue_4 (`self.DynamicMeshComponent`) (struct) null))))))

(fn `UserConstructionScript`)