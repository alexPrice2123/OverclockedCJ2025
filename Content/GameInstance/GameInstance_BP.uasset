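; GameInstance_BP is the game instance that persists a FirstHumanTime value between sessions through a SaveBP save slot.
; On Init it loads the existing save and restores the value, or creates and writes a new save, then prints the value.
; On Shutdown it copies FirstHumanTime back into the save object and writes it to the slot, provided a save already exists.
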(event `self.ReceiveShutdown`
  (bind _returnvalue (`GameplayStatics.DoesSaveGameExist` (`self.Slot Name`)))
  (if _returnvalue
    (set `/Game/GameInstance/SaveBP.Saved_FirstHumanTime` (`self.FirstHumanTime`) (`self.As Save BP`))
    (`GameplayStatics.SaveGameToSlot` (`self.As Save BP`) (`self.Slot Name`))))

(event `self.ReceiveInit`
  (bind _returnvalue (`GameplayStatics.DoesSaveGameExist` (`self.Slot Name`)))
  (if _returnvalue
    (bind _returnvalue_2 (`GameplayStatics.LoadGameFromSlot` (`self.Slot Name`)))
    (bind _assave_bp (cast `/Game/GameInstance/SaveBP` _returnvalue_2))
    (bind _output_get (set `self.As Save BP` _assave_bp))
    (set `self.FirstHumanTime` (`/Game/GameInstance/SaveBP.Saved_FirstHumanTime` _output_get))
    (else
      (bind _returnvalue_3 (`GameplayStatics.CreateSaveGameObject` "/Game/GameInstance/SaveBP.SaveBP_C"))
      (bind _output_get_2 (set `self.As Save BP` _returnvalue_3))
      (`GameplayStatics.SaveGameToSlot` _output_get_2 (`self.Slot Name`))))
  (`KismetSystemLibrary.PrintString` (`KismetStringLibrary.Conv_BoolToString` (`self.FirstHumanTime`))))